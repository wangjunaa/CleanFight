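; BP_BaseProp is a pickup prop that gives the character who picks it up a weapon with randomized modules.
; OnPickUp spawns PropActorClass as a Weapon at the world origin and sets the character as its owner.
; It rolls a module count, then spawns and attaches that many random module classes supplied by BP_GameSate.
; It passes the weapon to the character's WeaponComponent and destroys itself only if AddWeapon succeeds.
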(event `self.OnPickUp`
  (params (Character :type "BaseCharacter Object Reference"))
  (`KismetSystemLibrary.PrintString` "Hello")
  (`|ExecutionSequence`
    (:`then_0`
      ;[1 1 1] 生成武器
      (bind _returnvalue (`|SpawnActorFromClass` (`self.PropActorClass`) (`KismetMathLibrary.MakeTransform` (0.0 0.0 0.0)) "Undefined" "MultiplyWithRoot" null null))
      (bind _asweapon (cast `Weapon` _returnvalue))
      (bind _output_get (set `self.NewWeapon` _asweapon))
      (`self.SetOwner` _output_get Character))
    (:`then_1`
      ;[1 1 1] 添加随机模组
      (bind _output_get_2 (set `self.ModuleNum` (`KismetMathLibrary.RandomIntegerInRange` 1 6)))
      (`Weapon.SetMaxModuleNumber` (`self.NewWeapon`) _output_get_2)
      (bind _asbp_game_sate (cast `/Game/Blueprint/BP_GameSate` (`GameplayStatics.GetGameState`)))
      (for _ (range 1 (+ (`self.ModuleNum`) 1))
        (bind _moduleclass (`/Game/Blueprint/BP_GameSate.GetRandomWeaponModule` _asbp_game_sate))
        (bind _returnvalue_2 (`|SpawnActorFromClass` _moduleclass (`KismetMathLibrary.MakeTransform` (0.0 0.0 0.0)) "Undefined" "MultiplyWithRoot" null null))
        (`Weapon.AddModule` (`self.NewWeapon`) _returnvalue_2 -1)))
    (:`then_2`
      ;[1 1 1] 将武器给到角色
      (bind _returnvalue_3 (`WeaponComponent.AddWeapon` (`BaseCharacter.WeaponComponent` Character) (`self.NewWeapon`)))
      (if _returnvalue_3
        (`self.K2_DestroyActor`)
        (`KismetSystemLibrary.PrintString` "Hello")))))

(fn `UserConstructionScript`)