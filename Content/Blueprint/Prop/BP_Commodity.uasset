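; BP_Commodity is a weapon for sale, displaying a spawned instance of its WeaponClass on a Scene component.
; Highlighting spawns a second copy with every material swapped for a highlight instance, and un-highlighting destroys it.
; Sale spawns a fresh weapon, rolls its module capacity, adds random modules from BP_GameSate and offers it to the character's WeaponComponent.
; A successful add destroys the display weapon, highlight copy and capsule.
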(event `self.ReceiveBeginPlay`
  (bind _returnvalue (`|SpawnActorFromClass` (`self.WeaponClass`) (`KismetMathLibrary.MakeTransform` (0.0 0.0 0.0)) "Undefined" "MultiplyWithRoot" null null))
  (bind _output_get (set `self.Weapon` _returnvalue))
  (`SceneComponent.K2_AttachToComponent` (`Actor.RootComponent` _output_get) (`self.Scene`) "None" "KeepRelative" "KeepRelative" "KeepRelative" true))

(event `self.ReceiveTick`
  (params (DeltaSeconds :type "Float (single-precision)")))

(event `HightLightOn`
  (bind _returnvalue (`Weapon.GetMesh` (`self.HighLightMesh`)))
  (`self.Weapon`
    (:`then`
      (if (not (`self.IsHighLight`))
        (bind _returnvalue_2 (`|SpawnActorFromClass` (`self.WeaponClass`) (`KismetMathLibrary.MakeTransform` (0.0 0.0 0.0)) "Undefined" "MultiplyWithRoot" null null))
        (bind _output_get (set `self.HighLightMesh` _returnvalue_2))
        (`SceneComponent.K2_AttachToComponent` (`Actor.RootComponent` _output_get) (`self.Scene`) "None" "KeepRelative" "KeepRelative" "KeepRelative" true)
        (for (_ _array_index) (`MeshComponent.GetMaterials` _returnvalue)
          (`PrimitiveComponent.SetMaterial` _returnvalue _array_index "/Game/Material/HighLight_Inst.HighLight_Inst"))
        (set `self.IsHighLight` true)))
    (:`else`)))

(event `HighLightOff`
  (`self.Weapon`
    (:`then`
      (if (`self.IsHighLight`)
        (`self.K2_DestroyActor` (`self.HighLightMesh`))
        (set `self.IsHighLight` false)))
    (:`else`)))

(fn `Sale`
  (params (Character :type "BaseCharacter Object Reference"))
  (locals (NewWeapon :type "Weapon Object Reference"))
  (bind _returnvalue (`KismetMathLibrary.RandomIntegerInRange` 1 6))
  (`self.Weapon`
    (:`then`
      (bind _weaponcomponent (`BaseCharacter.WeaponComponent` Character)
        (:`then`
          (`|ExecutionSequence`
            (:`then_0`
              ;[1 1 1] 生成武器
              (bind _returnvalue_2 (`|SpawnActorFromClass` (`self.WeaponClass`) (`KismetMathLibrary.MakeTransform` (0.0 0.0 0.0)) "Undefined" "MultiplyWithRoot" null null))
              (set `local.NewWeapon` _returnvalue_2)
              (`self.SetOwner` Character))
            (:`then_1`
              ;[1 1 1] 添加随机模组
              (`Weapon.SetMaxModuleNumber` (`local.NewWeapon`) _returnvalue)
              (bind _asbp_game_sate (cast `/Game/Blueprint/BP_GameSate` (`GameplayStatics.GetGameState`)))
              (for _ (range 1 (+ (`KismetMathLibrary.RandomIntegerInRange` 1 _returnvalue) 1))
                (bind _moduleclass (`/Game/Blueprint/BP_GameSate.GetRandomModule` _asbp_game_sate))
                (bind _returnvalue_3 (`|SpawnActorFromClass` _moduleclass (`KismetMathLibrary.MakeTransform` (0.0 0.0 0.0)) "Undefined" "MultiplyWithRoot" null null))
                (`Weapon.AddModule` (`local.NewWeapon`) _returnvalue_3 -1)))
            (:`then_2`
              ;[1 1 1] 将武器给到角色
              (bind _returnvalue_4 (`WeaponComponent.AddWeapon` _weaponcomponent (`local.NewWeapon`)))
              (if _returnvalue_4
                (`self.K2_DestroyActor` (`self.HighLightMesh`))
                (`self.K2_DestroyActor` (`self.Weapon`))
                (`ActorComponent.K2_DestroyComponent` (`self.Capsule`))))))
        (:`else`)))
    (:`else`)))

(fn `UserConstructionScript`)