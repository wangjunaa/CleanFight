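; BP_GameSate is a helper Blueprint, apparently the game state, that supplies random modules and spawns the boss.
; Two getters each return a random entry from the weapon module list or the state module list.
; SpawnBoss spawns the configured boss class at the transform of player 0's pawn.
; The event graph and construction script hold no logic, so nothing runs until these functions are called.
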(fn `GetRandomStateModule`
  (returns (ModuleClass :type "StateModule Class Reference"))
  (return (`KismetArrayLibrary.Array_Random` (`self.StateModuleList`))))

(fn `GetRandomWeaponModule`
  (returns (ModuleClass :type "WeaponModule Class Reference"))
  (return (`KismetArrayLibrary.Array_Random` (`self.WeaponModuleList`))))

(fn `SpawnBoss`
  (`|SpawnActorFromClass` (`self.BossClass`) (`self.GetTransform` (`GameplayStatics.GetPlayerPawn` 0)) "Undefined" "MultiplyWithRoot" null null))

(fn `UserConstructionScript`)