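; BP_Enemy_NiLu is an enemy Blueprint that manages a floating health bar driven by its HealthComponent.
; BeginPlay caches the WB_HealthBar widget and hides it, then Tick copies the current health percent into it while the enemy is alive.
; Damage shows the bar, and a retriggerable delay hides it again a few seconds after the last hit.
; On death, Tick hides the bar once through a DoOnce.
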(event `self.ReceiveBeginPlay`
  (bind _aswb_health_bar (cast `/Game/UI/WB_HealthBar` (`WidgetComponent.GetUserWidgetObject` (`self.HealthBar`))))
  (set `self.As UW Health Bar` _aswb_health_bar)
  (`SceneComponent.SetVisibility` (`self.HealthBar`) false false))

(event `self.ReceiveTick`
  (params (DeltaSeconds :type "Float (single-precision)"))
  (bind _returnvalue (`self.GetComponentByClass` "/Script/CleanFight.HealthComponent"))
  (if (`HealthComponent.IsDeath` _returnvalue)
    (`/Engine/EditorBlueprintResources/StandardMacros.DoOnce` false
      (:`Completed`
        (`SceneComponent.SetVisibility` (`self.HealthBar`) false false)))
    (else
      (set `/Game/UI/WB_HealthBar.HealthPercent` (`HealthComponent.GetHealthPercent` _returnvalue) (`self.As UW Health Bar`)))))

(event `self.ReceiveAnyDamage`
  (params (Damage :type "Float (single-precision)") (DamageType :type "DamageType Object Reference") (InstigatedBy :type "Controller Object Reference") (DamageCauser :type "Actor Object Reference"))
  (if (not (`HealthComponent.IsDeath` (`self.GetComponentByClass` "/Script/CleanFight.HealthComponent")))
    (`SceneComponent.SetVisibility` (`self.HealthBar`) true false)
    (`KismetSystemLibrary.RetriggerableDelay` 3.0)
    (`SceneComponent.SetVisibility` (`self.HealthBar`) false false)))

(fn `UserConstructionScript`)