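; BP_Enemy is an enemy Blueprint that displays its health on a UW_HealthBar widget and hides the bar when it dies.
; BeginPlay casts and caches the user widget from its HealthBar widget component.
; Tick polls the HealthComponent, copying its health percent into the widget while alive and hiding the bar once through a DoOnce on death.
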(event `self.ReceiveBeginPlay`
  (bind _asuw_health_bar (cast `/Game/UI/UW_HealthBar` (`WidgetComponent.GetUserWidgetObject` (`self.HealthBar`))))
  (set `self.As UW Health Bar` _asuw_health_bar))

(event `self.ReceiveTick`
  (params (DeltaSeconds :type "Float (single-precision)"))
  (bind _returnvalue (`self.GetComponentByClass` "/Script/CleanFight.HealthComponent"))
  (if (`HealthComponent.IsDeath` _returnvalue)
    (`/Engine/EditorBlueprintResources/StandardMacros.DoOnce` false
      (:`Completed`
        (`SceneComponent.SetVisibility` (`self.HealthBar`) false false)))
    (else
      (set `/Game/UI/UW_HealthBar.HealthPercent` (`HealthComponent.GetHealthPercent` _returnvalue) (`self.As UW Health Bar`)))))

(fn `UserConstructionScript`)