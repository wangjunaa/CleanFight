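; Boss enemy that spawns with boosted max health and a modular weapon preloaded with speed-up and damage-up modules.
; BeginPlay links the health bar widget to its HealthComponent, equips the weapon through WeaponComponent and binds the death event.
; Damage reveals the health bar until a retriggerable delay hides it again, and Tick hides it once on death.
; Death also tints the level's directional light and calls the game state's BGM playback.
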(event `self.ReceiveBeginPlay`
  (bind _returnvalue (`KismetMathLibrary.MakeTransform` (0.0 0.0 0.0)))
  (`|ExecutionSequence`
    (:`then_0`
      (bind _aswbp_health_bar (cast `/Game/UI/Player/WBP_HealthBar` (`WidgetComponent.GetUserWidgetObject` (`self.HealthBar`))))
      (bind _output_get (set `self.As UW Health Bar` _aswbp_health_bar))
      (set `/Game/UI/Player/WBP_HealthBar.HealthComp` (`self.GetComponentByClass` "/Script/CleanFight.HealthComponent") _output_get)
      (`SceneComponent.SetVisibility` (`self.HealthBar`) false false)
      (bind _returnvalue_2 (`|SpawnActorFromClass` "/Game/Blueprint/Weapon/BP_Weapon_Init.BP_Weapon_Init_C" (`KismetMathLibrary.MakeTransform` (0.0 0.0 0.0)) "Undefined" "MultiplyWithRoot" null null))
      (`Weapon.SetMaxModuleNumber` _returnvalue_2 6)
      (`WeaponComponent.AddWeapon` (`self.WeaponComponent`) _returnvalue_2)
      (`HealthComponent.AddMaxHealth` (`self.HealthComponent`) 2000.0))
    (:`then_1`
      (for _ (range 3)
        (bind _returnvalue_3 (`|SpawnActorFromClass` "/Game/Blueprint/Weapon/Modules/WM_SpeedUp.WM_SpeedUp_C" _returnvalue "Undefined" "MultiplyWithRoot" null null))
        (`Weapon.AddModule` (`WeaponComponent.GetCurrentWeapon` (`self.WeaponComponent`)) _returnvalue_3 -1))
      (for _ (range 3)
        (bind _returnvalue_4 (`|SpawnActorFromClass` "/Game/Blueprint/Weapon/Modules/WM_DamgeUp.WM_DamgeUp_C" _returnvalue "Undefined" "MultiplyWithRoot" null null))
        (`Weapon.AddModule` (`WeaponComponent.GetCurrentWeapon` (`self.WeaponComponent`)) _returnvalue_4 -1)))
    (:`then_2`
      (add `HealthComponent.OnDeath` (`self.HealthComponent`) (delegate `OnDeath_事件`)))))

(event `OnDeath_事件`
  (params (Killer :type "Controller Object Reference"))
  (bind _returnvalue (`GameplayStatics.GetActorOfClass` "/Script/Engine.DirectionalLight"))
  (`LightComponent.SetLightColor` (`Light.LightComponent` _returnvalue) (struct :`R` 0.7 :`G` 0.5 :`B` 0.5 :`A` 1.0) true)
  (bind _asgs_level (cast `/Game/Blueprint/GS_Level` (`GameplayStatics.GetGameState`)))
  (`/Game/Blueprint/GS_Level.PlayBGM` _asgs_level))

(event `self.ReceiveTick`
  (params (DeltaSeconds :type "Float (single-precision)"))
  (if (`HealthComponent.IsDeath` (`self.GetComponentByClass` "/Script/CleanFight.HealthComponent"))
    (`/Engine/EditorBlueprintResources/StandardMacros.DoOnce` false
      (:`Completed`
        (`SceneComponent.SetVisibility` (`self.HealthBar`) false false)))))

(event `self.ReceiveAnyDamage`
  (params (Damage :type "Float (single-precision)") (DamageType :type "DamageType Object Reference") (InstigatedBy :type "Controller Object Reference") (DamageCauser :type "Actor Object Reference"))
  (if (not (`HealthComponent.IsDeath` (`self.GetComponentByClass` "/Script/CleanFight.HealthComponent")))
    (`SceneComponent.SetVisibility` (`self.HealthBar`) true false)
    (`KismetSystemLibrary.RetriggerableDelay` 3.0)
    (`SceneComponent.SetVisibility` (`self.HealthBar`) false false)))

(fn `UserConstructionScript`)