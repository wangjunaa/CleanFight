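; GM_Level_Multi is a multiplayer level GameMode that spawns and possesses a BP_NiLu pawn for each joining player.
; BeginPlay caches PlayerStarts; PostLogin records the controller and, after a short delay, spawns at the saved transform if a save is loaded, otherwise at the PlayerStart matching join order.
; LoadGame reads the "Level" save slot, spawns enemies at saved transforms and restores game time on BaseGameState.
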(event `self.ReceiveBeginPlay`
  (bind _outactors (`GameplayStatics.GetAllActorsOfClass` "/Script/Engine.PlayerStart"))
  (set `self.PlayerStarts` _outactors))

(event `self.K2_PostLogin`
  (params (NewPlayer :type "PlayerController Object Reference"))
  (bind _asbp_player_controller (cast `/Game/Blueprint/Character/NiLu/BP_PlayerController` NewPlayer)
    (:`then`
      (set `self.CurrentLoginPlayerController` _asbp_player_controller)
      (bind _returnvalue (`KismetArrayLibrary.Array_Add` (`self.Player Controllers`) _asbp_player_controller))
      (`KismetSystemLibrary.Delay` 0.2)
      (bind _save_level (`self.Save Level`)
        (:`then`
          (bind _returnvalue_2 (`|SpawnActorFromClass` "/Game/Blueprint/Character/NiLu/BP_NiLu.BP_NiLu_C" (`/Game/Save/Save_Level.NiLuTransform` _save_level) "Undefined" "MultiplyWithRoot" null (`self.CurrentLoginPlayerController`) null))
          (`Controller.Possess` (`self.CurrentLoginPlayerController`) _returnvalue_2))
        (:`else`
          (bind (_returnvalue_location _returnvalue_rotation) (`KismetMathLibrary.BreakTransform` (`self.GetTransform` (`|GetArrayItem` (`self.PlayerStarts`) _returnvalue))))
          (bind _returnvalue_3 (`|SpawnActorFromClass` "/Game/Blueprint/Character/NiLu/BP_NiLu.BP_NiLu_C" (`KismetMathLibrary.MakeTransform` _returnvalue_location _returnvalue_rotation) "Undefined" "MultiplyWithRoot" null (`self.CurrentLoginPlayerController`) null))
          (`Controller.Possess` (`self.CurrentLoginPlayerController`) _returnvalue_3)))
      (`KismetSystemLibrary.PrintString` "玩家加入"))
    (:`CastFailed`
      (`KismetSystemLibrary.PrintString` "加入失败"))))

(event `LoadGame`
  (bind _returnvalue (`GameplayStatics.LoadGameFromSlot` "Level"))
  (bind _assave_level (cast `/Game/Save/Save_Level` _returnvalue))
  (set `self.Save Level` _assave_level)
  (`KismetSystemLibrary.PrintString` "加载游戏存档")
  (for _array_element (`/Game/Save/Save_Level.EnemyTransform` (`self.Save Level`))
    (`|SpawnActorFromClass` "/Game/Blueprint/Enemy/BP_Enemy_NiLu.BP_Enemy_NiLu_C" _array_element "Undefined" "MultiplyWithRoot" null null))
  (bind _asbase_game_state (cast `BaseGameState` (`GameplayStatics.GetGameState`)))
  (`BaseGameState.SetTime` _asbase_game_state (`/Game/Save/Save_Level.GameTime` (`self.Save Level`))))

(fn `UserConstructionScript`)