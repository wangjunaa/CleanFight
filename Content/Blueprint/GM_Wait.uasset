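; Game mode for a multiplayer waiting room that tracks joined and ready players before travel to Level_SinglePlayer.
; PostLogin stores each controller, creates its wait UI and, after a short delay, spawns and possesses a BP_NiLu at the PlayerStart matching its join index.
; Player and ready counts are copied to GS_Wait.
; EntryLevel issues the servertravel command once for every stored controller.
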(event `self.ReceiveBeginPlay`
  (bind _outactors (`GameplayStatics.GetAllActorsOfClass` "/Script/Engine.PlayerStart"))
  (set `self.PlayerStarts` _outactors))

(event `self.K2_PostLogin`
  (params (NewPlayer :type "PlayerController Object Reference"))
  (bind _asbp_player_controller_wait (cast `/Game/Blueprint/Character/NiLu/BP_PlayerController_Wait` NewPlayer))
  (`|ExecutionSequence`
    (:`then_0`
      (bind _returnvalue (`KismetArrayLibrary.Array_Add` (`self.PlayerControllers`) _asbp_player_controller_wait))
      (`KismetSystemLibrary.Delay` 0.2)
      (bind (_returnvalue_location _returnvalue_rotation) (`KismetMathLibrary.BreakTransform` (`self.GetTransform` (`|GetArrayItem` (`self.PlayerStarts`) _returnvalue))))
      (bind _returnvalue_2 (`|SpawnActorFromClass` "/Game/Blueprint/Character/NiLu/BP_NiLu.BP_NiLu_C" (`KismetMathLibrary.MakeTransform` _returnvalue_location _returnvalue_rotation) "Undefined" "MultiplyWithRoot" null _asbp_player_controller_wait null))
      (`Controller.Possess` _asbp_player_controller_wait _returnvalue_2)
      (`KismetSystemLibrary.PrintString` "玩家加入"))
    (:`then_1`
      (`/Game/Blueprint/Character/NiLu/BP_PlayerController_Wait.CreateWaitUI` _asbp_player_controller_wait)
      (bind _asgs_wait (cast `/Game/Blueprint/GS_Wait` (`GameplayStatics.GetGameState`)))
      (set `/Game/Blueprint/GS_Wait.PlayerNum` (`KismetArrayLibrary.Array_Length` (`self.PlayerControllers`)) _asgs_wait))))

(event `AddReadyPlayer`
  (bind _output_get (set `self.ReadyNum` (+ (`self.ReadyNum`) 1)))
  (bind _asgs_wait (cast `/Game/Blueprint/GS_Wait` (`GameplayStatics.GetGameState`)))
  (set `/Game/Blueprint/GS_Wait.ReadyNum` _output_get _asgs_wait))

(event `RemoveReady`
  (bind _output_get (set `self.ReadyNum` (- (`self.ReadyNum`) 1)))
  (bind _asgs_wait (cast `/Game/Blueprint/GS_Wait` (`GameplayStatics.GetGameState`)))
  (set `/Game/Blueprint/GS_Wait.ReadyNum` _output_get _asgs_wait))

(event `EntryLevel`
  (for _array_element (`self.PlayerControllers`)
    (`KismetSystemLibrary.ExecuteConsoleCommand` "servertravel /Game/Level/Level_SinglePlayer" _array_element)))

(fn `UserConstructionScript`)