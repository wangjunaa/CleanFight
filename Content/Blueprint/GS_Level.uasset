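; GS_Level is a level Game State Blueprint that serves random modules and exposes background music controls.
; Two getters return random entries from the weapon module and state module lists.
; PlayBGM and StopBGM look up the BGM_Loop actor by class and forward the call when it is valid.
; BeginPlay, Tick and the construction script hold no logic.
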(event `self.ReceiveBeginPlay`)

(fn `GetRandomStateModule`
  (returns (ModuleClass :type "StateModule Class Reference"))
  (return (`KismetArrayLibrary.Array_Random` (`self.StateModuleList`))))

(fn `GetRandomWeaponModule`
  (returns (ModuleClass :type "WeaponModule Class Reference"))
  (return (`KismetArrayLibrary.Array_Random` (`self.WeaponModuleList`))))

(fn `PlayBGM`
  (bind _returnvalue (`GameplayStatics.GetActorOfClass` "/Game/Audio/BGM/BGM_Loop.BGM_Loop_C"))
  (`/Engine/EditorBlueprintResources/StandardMacros.IsValid` _returnvalue
    (:`Is Valid`
      (`/Game/Audio/BGM/BGM_Loop.PlayBGM` _returnvalue))))

(fn `StopBGM`
  (bind _returnvalue (`GameplayStatics.GetActorOfClass` "/Game/Audio/BGM/BGM_Loop.BGM_Loop_C"))
  (`/Engine/EditorBlueprintResources/StandardMacros.IsValid` _returnvalue
    (:`Is Valid`
      (`/Game/Audio/BGM/BGM_Loop.StopBGM` _returnvalue))))

(fn `UserConstructionScript`)