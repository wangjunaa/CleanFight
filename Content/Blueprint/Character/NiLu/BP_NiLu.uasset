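; BP_NiLu is the NiLu player character, with a healing Q skill and a shield E skill bound to input actions.
; Q attaches a Niagara heal effect to the spine and adds health; E spawns a shield actor, destroyed after a delay.
; Tick counts down both cooldowns while alive and getters expose their remaining fraction.
; The health component's death event is forwarded to BP_PlayerController.
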(event `self.ReceiveBeginPlay`
  (add `HealthComponent.OnDeath` (`self.HealthComponent`) (`|CreateDelegate` :!event `OnDeath_事件`)))

(event `SpawnVFX`
  (`NiagaraFunctionLibrary.SpawnSystemAttached` "/Game/Effect/VFX/NS_Heal.NS_Heal" (`self.Mesh`) "Character1_Spine" (0.0 0.0 0.0) (struct :`Roll` 90.0) "KeepRelativeOffset" true))

(event `self.ReceiveTick`
  (params (DeltaSeconds :type "Float (single-precision)"))
  (if (not (`HealthComponent.IsDeath` (`self.HealthComponent`)))
    (`self.CDTImer` DeltaSeconds)))

(event `Skill_Q`
  ;[1 1 1] Q技能
  (if (not (`self.InCD_Q`))
    (`self.SpawnVFX`)
    (`HealthComponent.AddHealth` (`self.HealthComponent`) 50.0)
    (set `self.InCD_Q` true)
    (set `self.ResCD_Q` (`self.CD_Q`))))

(event `EnhancedInput|/Game/Input/IA/IA_Q`
  (params (ActionValue :type Boolean) (ElapsedSeconds :type "Float (double-precision)") (TriggeredSeconds :type "Float (double-precision)") (InputAction :type "InputAction Object Reference" :default "/Game/Input/IA/IA_Q.IA_Q"))
  (:`Started`
    (`self.Skill_Q`)))

(event `Skill_E`
  ;[1 1 1] E技能
  (if (not (`self.InCD_E`))
    (bind _returnvalue (`|SpawnActorFromClass` "/Game/Blueprint/Prop/BP_Shield.BP_Shield_C" (`self.GetTransform`) "Undefined" "MultiplyWithRoot" null null))
    (set `self.InCD_E` true)
    (set `self.ResCD_E` (`self.CD_E`))
    (`KismetSystemLibrary.Delay` 10.0)
    (`self.K2_DestroyActor` _returnvalue)))

(event `EnhancedInput|/Game/Input/IA/IA_E`
  (params (ActionValue :type Boolean) (ElapsedSeconds :type "Float (double-precision)") (TriggeredSeconds :type "Float (double-precision)") (InputAction :type "InputAction Object Reference" :default "/Game/Input/IA/IA_E.IA_E"))
  (:`Started`
    (`self.Skill_E`)))

(event `self.ReceiveAnyDamage`
  (params (Damage :type "Float (single-precision)") (DamageType :type "DamageType Object Reference") (InstigatedBy :type "Controller Object Reference") (DamageCauser :type "Actor Object Reference")))

(event `OnDeath_事件`
  (params (Killer :type "Controller Object Reference"))
  (bind _asbp_player_controller (cast `/Game/Blueprint/Character/NiLu/BP_PlayerController` (`self.GetController`))
    (:`then`
      (`/Game/Blueprint/Character/NiLu/BP_PlayerController.OnDeath` _asbp_player_controller))
    (:`CastFailed`
      (`KismetSystemLibrary.PrintString` "BP_Nilu OnDeath:无控制"))))

(fn `CDTImer`
  (params (Delta :type "Float (double-precision)"))
  (locals (DeltaTime :type "Float (double-precision)"))
  (set `local.DeltaTime` Delta)
  (`|ExecutionSequence`
    (:`then_0`
      (if (`self.InCD_Q`)
        (bind _output_get (set `self.ResCD_Q` (- (`self.ResCD_Q`) (`local.DeltaTime`))))
        (if (<= _output_get 0.0)
          (set `self.InCD_Q` false))))
    (:`then_1`
      (if (`self.InCD_E`)
        (bind _output_get_2 (set `self.ResCD_E` (- (`self.ResCD_E`) (`local.DeltaTime`))))
        (if (<= _output_get_2 0.0)
          (set `self.InCD_E` false))))))

(fn `GetCDPercent_E`
  (returns (Percent :type "Float (double-precision)"))
  (return (/ (`self.ResCD_E`) (`self.CD_E`))))

(fn `GetCDPercent_Q`
  (returns (Percent :type "Float (double-precision)"))
  (return (/ (`self.ResCD_Q`) (`self.CD_Q`))))

(fn `UserConstructionScript`)