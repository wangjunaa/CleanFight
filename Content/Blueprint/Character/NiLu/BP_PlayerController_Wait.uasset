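; Player controller for a waiting screen, where players mark themselves ready or not ready.
; CreateWaitUI creates a WBP_Wait widget after a short delay and adds it to the viewport.
; Ready and UnReady cast the game mode to GM_Wait and call its AddReadyPlayer and RemoveReady, leaving the ready tracking to the game mode.
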(event `self.ReceiveBeginPlay`)

(event `self.ReceiveTick`
  (params (DeltaSeconds :type "Float (single-precision)")))

(event `CreateWaitUI`
  (`KismetSystemLibrary.Delay` 0.2)
  (bind _returnvalue (`|CreateWidget` "/Game/UI/GameUI/WBP_Wait.WBP_Wait_C" self (not (`self.HasAuthority`))))
  (`UserWidget.AddToViewport` _returnvalue 0))

(event `Ready`
  (bind _asgm_wait (cast `/Game/Blueprint/GM_Wait` (`GameplayStatics.GetGameMode`)))
  (`/Game/Blueprint/GM_Wait.AddReadyPlayer` _asgm_wait))

(event `UnReady`
  (bind _asgm_wait (cast `/Game/Blueprint/GM_Wait` (`GameplayStatics.GetGameMode`)))
  (`/Game/Blueprint/GM_Wait.RemoveReady` _asgm_wait))

(fn `UserConstructionScript`)