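; Player controller that manages UI, the starting weapon and item pickup for the BP_NiLu character.
; After a startup delay it creates the HUD and adds an initial weapon to the pawn's WeaponComponent.
; A per-tick box trace from the viewpoint highlights the PickUpProp ahead, which F picks up.
; Tab opens the bag with UI-only input, while OnDeath shows the death screen and removes the HUD and bag.
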(event `self.ReceiveBeginPlay`
  (`KismetSystemLibrary.Delay` 3.0)
  (`self.CreatePlayerUI`)
  (`self.SpawnInitWeapon`))

(event `self.ReceiveTick`
  (params (DeltaSeconds :type "Float (single-precision)"))
  (`self.WatchingTrace`))

(event `CreatePlayerUI`
  (`KismetSystemLibrary.Delay` 0.2)
  (bind _returnvalue (`|CreateWidget` "/Game/UI/Player/WBP_Player.WBP_Player_C" self))
  (bind _output_get (set `self.PlayerUI` _returnvalue))
  (`UserWidget.AddToViewport` _output_get 0))

(event `SpawnInitWeapon`
  (bind _returnvalue (`self.K2_GetPawn`))
  (bind _asbp_ni_lu (cast `/Game/Blueprint/Character/NiLu/BP_NiLu` _returnvalue)
    (:`then`
      (bind _returnvalue_2 (`|SpawnActorFromClass` "/Game/Blueprint/Weapon/BP_Weapon_Init.BP_Weapon_Init_C" (`KismetMathLibrary.MakeTransform` (0.0 0.0 0.0)) "Undefined" "MultiplyWithRoot" _returnvalue null))
      (bind _returnvalue_3 (`WeaponComponent.AddWeapon` (`BaseCharacter.WeaponComponent` _asbp_ni_lu) _returnvalue_2))
      (if _returnvalue_3
        (`KismetSystemLibrary.PrintString` "生成武器成功")))
    (:`CastFailed`
      (`KismetSystemLibrary.PrintString` "生成初始武器失败"))))

(event `OnDeath`
  (`|ExecutionSequence`
    (:`then_0`
      (bind _returnvalue (`|CreateWidget` "/Game/UI/Player/WBP_DeathUI.WBP_DeathUI_C" self))
      (`UserWidget.AddToViewport` _returnvalue 0)
      (set `PlayerController.bShowMouseCursor` true))
    (:`then_1`
      (bind _playerui (`self.PlayerUI`)
        (:`then`
          (`Widget.RemoveFromParent` _playerui)
          (bind _bagui (`self.BagUI`)
            (:`then`
              (`Widget.RemoveFromParent` _bagui))
            (:`else`)))
        (:`else`)))))

(event `EnhancedInput|/Game/Input/IA/IA_Tab`
  (params (ActionValue :type Boolean) (ElapsedSeconds :type "Float (double-precision)") (TriggeredSeconds :type "Float (double-precision)") (InputAction :type "InputAction Object Reference" :default "/Game/Input/IA/IA_Tab.IA_Tab"))
  (:`Started`
    (bind _returnvalue (`|CreateWidget` "/Game/UI/Bag/WBP_BagMain.WBP_BagMain_C" self (`self.PlayerUI`)))
    (bind _output_get (set `self.BagUI` _returnvalue))
    (`UserWidget.AddToViewport` _output_get 10)
    (`WidgetBlueprintLibrary.SetInputMode_UIOnlyEx` self (`self.BagUI`) "DoNotLock" true)
    (set `PlayerController.bShowMouseCursor` true)))

(event `WatchingTrace`
  (bind (_location _rotation) (`self.GetPlayerViewPoint` self))
  (`/Engine/EditorBlueprintResources/StandardMacros.IsValid` self
    (:`Is Valid`
      (bind _outhit (`KismetSystemLibrary.BoxTraceSingleForObjects` _location (+ _location (* (`KismetMathLibrary.GetForwardVector` _rotation) 200)) (10.0 10.0 10.0) (struct) (`|MakeArray` "ObjectTypeQuery2" :!type "EObjectTypeQuery Enum")))
      (bind _watchingpickup (`self.WatchingPickUp`)
        (:`then`
          (`PickUpProp.HighLightOff` _watchingpickup))
        (:`else`
          _))
      (bind (_bblockinghit _binitialoverlap _time _distance _location_2 _impactpoint _normal _impactnormal _physmat _hitactor) (`GameplayStatics.BreakHitResult` _outhit))
      (if _bblockinghit
        (bind _aspick_up_prop (cast `PickUpProp` _hitactor))
        (bind _output_get (set `self.WatchingPickUp` _aspick_up_prop))
        (`PickUpProp.HighLightOn` _output_get)
        (else
          (set `self.WatchingPickUp` _watchingpickup))))
    (:`Is Not Valid`
      (`KismetSystemLibrary.PrintString` "盒体检测无控制者"))))

(event `EnhancedInput|/Game/Input/IA/IA_F`
  (params (ActionValue :type Boolean) (ElapsedSeconds :type "Float (double-precision)") (TriggeredSeconds :type "Float (double-precision)") (InputAction :type "InputAction Object Reference" :default "/Game/Input/IA/IA_F.IA_F"))
  (:`Started`
    (`self.PickUp`)))

(event `PickUp`
  (bind _watchingpickup (`self.WatchingPickUp`)
    (:`then`
      (bind _asbp_ni_lu (cast `/Game/Blueprint/Character/NiLu/BP_NiLu` (`self.K2_GetPawn` self)))
      (`PickUpProp.OnPickUp` _watchingpickup _asbp_ni_lu))
    (:`else`)))

(fn `UserConstructionScript`)